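; Camera pawn that acts as a paint brush for BP_MapPoint map points, with the system mouse cursor hidden.
; Each tick moves the Brush to the Visibility trace hit under the cursor, while held bracket keys shrink or grow it through looping timers.
; Left click paints every point in ActivePoints and sets IsPainting until release clears PaintedList.
; Public-style add and remove functions maintain both lists, with no callers in this graph.
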(event `self.ReceiveBeginPlay`
  (set `PlayerController.bShowMouseCursor` false (`GameplayStatics.GetPlayerController` 0)))

(event `self.ReceiveTick`
  (params (DeltaSeconds :type "Float (single-precision)"))
  (`self.UpdateBrushPosition`))

(event `Key|LeftBracket`
  (params (Key :type "Key Structure"))
  ;[1 1 1] Brush Scale
  (:`Pressed`
    (bind _returnvalue (`KismetSystemLibrary.K2_SetTimerDelegate` (delegate `ScaleUpBrush`) 0.01 true)))
  (:`Released`
    (`KismetSystemLibrary.K2_ClearAndInvalidateTimerHandle` _returnvalue)))

(event `ScaleUpBrush`
  ;[1 1 1] Brush Scale
  (`self.BrushScale` 0.98))

(event `Key|RightBracket`
  (params (Key :type "Key Structure"))
  ;[1 1 1] Brush Scale
  (:`Pressed`
    (bind _returnvalue (`KismetSystemLibrary.K2_SetTimerDelegate` (delegate `ScaleDownBrush`) 0.01 true)))
  (:`Released`
    (`KismetSystemLibrary.K2_ClearAndInvalidateTimerHandle` _returnvalue)))

(event `ScaleDownBrush`
  ;[1 1 1] Brush Scale
  (`self.BrushScale` 1.02))

(event `Key|LeftMouseButton`
  (params (Key :type "Key Structure"))
  (:`Pressed`
    (set `self.IsPainting` true)
    (bind _output_get (set `self.PaintedList` (`self.ActivePoints`)))
    (for _array_element _output_get
      (`/Game/Blueprints/SceneBuild/BP_MapPoint.Paint` (cast `/Game/Blueprints/SceneBuild/BP_MapPoint` _array_element :!pure true))))
  (:`Released`
    (set `self.IsPainting` false)
    (`KismetArrayLibrary.Array_Clear` (`self.PaintedList`))))

(fn `AddPointToActiveList`
  (params (Point :type "Actor Object Reference (by ref)"))
  (`KismetArrayLibrary.Array_AddUnique` (`self.ActivePoints`) Point))

(fn `AddPointToPaintedList`
  (params (Point :type "Actor Object Reference (by ref)"))
  (`KismetArrayLibrary.Array_Add` (`self.PaintedList`) Point))

(fn `BrushScale`
  (params (Scale :type "Float (double-precision)"))
  (bind (_returnvalue_location _returnvalue_rotation _returnvalue_scale) (`KismetMathLibrary.BreakTransform` (`SceneComponent.GetRelativeTransform` (`self.Brush`))))
  (`SceneComponent.SetRelativeScale3D` (`self.Brush`) (* _returnvalue_scale Scale)))

(fn `RemovePointFromActiveList`
  (params (Point :type "Actor Object Reference (by ref)"))
  (`KismetArrayLibrary.Array_RemoveItem` (`self.ActivePoints`) Point))

(fn `UpdateBrushPosition`
  (`SceneComponent.K2_SetWorldLocation` (`self.Brush`) (`.Location` (`GameplayStatics.BreakHitResult` (`PlayerController.GetHitResultUnderCursorByChannel` (`GameplayStatics.GetPlayerController` 0) "TraceTypeQuery1" true))) false false))

(fn `UserConstructionScript`)