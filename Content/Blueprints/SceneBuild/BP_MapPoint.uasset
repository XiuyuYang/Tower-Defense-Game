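; BP_MapPoint is a paintable height point in a tile map, shared by tiles stored by corner.
; Overlap with the player's BP_CameraPawn highlights its cube via custom primitive data, updates the pawn's active list and, while painting, paints it once per painted list.
; Painting in Up mode, if every neighbouring BP_MapTile validates, raises the point a step and notifies those tiles.
; An optional debug text shows the height.
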(event `self.Cube.OnComponentBeginOverlap`
  (params (OverlappedComponent :type "PrimitiveComponent Object Reference") (OtherActor :type "Actor Object Reference") (OtherComp :type "PrimitiveComponent Object Reference") (OtherBodyIndex :type Integer) (bFromSweep :type Boolean) (SweepResult :type "HitResult Structure (by ref)"))
  (bind _returnvalue (`GameplayStatics.GetPlayerPawn` 0))
  (bind _asbp_camera_pawn (cast `/Game/Blueprints/GameBlueprints/BP_CameraPawn` _returnvalue :!pure true))
  (if (== _returnvalue OtherActor)
    (`PrimitiveComponent.SetCustomPrimitiveDataFloat` (`self.Cube`) 0 1.0)
    (`/Game/Blueprints/GameBlueprints/BP_CameraPawn.AddPointToActiveList` _asbp_camera_pawn self)
    (if (and (`/Game/Blueprints/GameBlueprints/BP_CameraPawn.IsPainting` _asbp_camera_pawn) (not (`KismetArrayLibrary.Array_Contains` (`/Game/Blueprints/GameBlueprints/BP_CameraPawn.PaintedList` _asbp_camera_pawn) self)))
      (`self.Paint`)
      (`/Game/Blueprints/GameBlueprints/BP_CameraPawn.AddPointToPaintedList` _asbp_camera_pawn self))))

(event `self.Cube.OnComponentEndOverlap`
  (params (OverlappedComponent :type "PrimitiveComponent Object Reference") (OtherActor :type "Actor Object Reference") (OtherComp :type "PrimitiveComponent Object Reference") (OtherBodyIndex :type Integer))
  (bind _returnvalue (`GameplayStatics.GetPlayerPawn` 0))
  (if (== _returnvalue OtherActor)
    (`PrimitiveComponent.SetCustomPrimitiveDataFloat` (`self.Cube`) 0 0.0)
    (`/Game/Blueprints/GameBlueprints/BP_CameraPawn.RemovePointFromActiveList` (cast `/Game/Blueprints/GameBlueprints/BP_CameraPawn` _returnvalue :!pure true) self)))

(event `Paint`
  (bind _canpaint (`self.CheckPaintValid`))
  (if _canpaint
    (switch `/Game/Blueprints/SceneBuild/EN_BrushMode` (`/Game/Blueprints/GameBlueprints/BP_CameraPawn.BrushMode` (cast `/Game/Blueprints/GameBlueprints/BP_CameraPawn` (`GameplayStatics.GetPlayerPawn` 0) :!pure true))
      (:`NewEnumerator0`
        (`self.PaintUp`)
        (bind _values (`BlueprintMapLibrary.Map_Values` (`self.Tiles`)))
        (for _array_element _values
          (`/Game/Blueprints/SceneBuild/BP_MapTile.ChangeHightness` (cast `/Game/Blueprints/SceneBuild/BP_MapTile` _array_element :!pure true) self))))))

(fn `CheckPaintMode`
  (params (Mode :type "/Game/Blueprints/SceneBuild/EN_BrushMode Enum" :default "NewEnumerator3"))
  (returns (ReturnValue :type Boolean))
  (return (`|EnumEquality` (`/Game/Blueprints/GameBlueprints/BP_CameraPawn.BrushMode` (cast `/Game/Blueprints/GameBlueprints/BP_CameraPawn` (`GameplayStatics.GetPlayerPawn` 0) :!pure true)) Mode)))

(fn `CheckPaintValid`
  (returns (CanPaint :type Boolean))
  (locals (CanPaintUp :type "Array of Boolean"))
  (bind _enumvalue (foreach `/Game/Blueprints/SceneBuild/EN_TileCorners` false)
    (:`LoopBody`
      (bind (_value _returnvalue) (`BlueprintMapLibrary.Map_Find` (`self.Tiles`) _enumvalue))
      (if _returnvalue
        (bind _canpaintup (`/Game/Blueprints/SceneBuild/BP_MapTile.PaintValidate` (cast `/Game/Blueprints/SceneBuild/BP_MapTile` _value :!pure true) self))
        (if (not _canpaintup)
          (return false))))
    (:`then`
      (return true))))

(fn `PaintUp`
  (`/Engine/EditorBlueprintResources/StandardMacros.IncrementInt` (`self.Hightness`)
    (:`  `
      (`SceneComponent.K2_AddLocalOffset` (`self.Cube`) (0.0 0.0 50.0) false false)
      (`self.ShowDebug`))))

(fn `ShowDebug`
  (if (`self.IsDebugging`)
    (`TextRenderComponent.K2_SetText` (`self.TextRender`) (`KismetTextLibrary.Conv_IntToText` (`self.Hightness`)))
    (`SceneComponent.K2_SetRelativeLocation` (`self.TextRender`) (`KismetMathLibrary.MakeVector` 0.0 0.0 (`KismetMathLibrary.Conv_IntToDouble` (+ (* (`self.Hightness`) 50) 10))) false false)))

(fn `UserConstructionScript`
  (`SceneComponent.SetVisibility` (`self.DebugActor`) (`self.IsDebugging`) true))