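; BP_MapEdge is a scene-building actor for a map edge, configured as either a left/right or an up/down type.
; Its construction script rotates the Cube 90 degrees for the up/down type.
; A debug flag toggles DebugActor and its children, with two text labels naming the sides to match the type.
; The event graph holds no active logic.
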(fn `UserConstructionScript`
  (bind _debugactor (`self.DebugActor`))
  (if (not (`self.LeftRightType`))
    (`SceneComponent.K2_SetRelativeRotation` (`self.Cube`) (struct :`Yaw` 90.0) false false))
  (if (`self.IsDebugging`)
    (`SceneComponent.SetVisibility` _debugactor true true)
    (if (`self.LeftRightType`)
      (`TextRenderComponent.K2_SetText` (`self.Text_Left/Up`) "Left")
      (`TextRenderComponent.K2_SetText` (`self.Text_Right/Down`) "Right")
      (else
        (`TextRenderComponent.K2_SetText` (`self.Text_Left/Up`) "Up")
        (`TextRenderComponent.K2_SetText` (`self.Text_Right/Down`) "Down")))
    (else
      (`SceneComponent.SetVisibility` _debugactor false true))))