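; Terrain map tile actor that tracks four corner heights and swaps its mesh to match as points are raised.
; ChangeHightness raises matching corners, then UpdateHightness rebases them to zero, moving the shared minimum into tile Z offset.
; UpdateMesh keys a proxy DataTable by concatenated corner heights, yielding yaw and a mesh row in the camera pawn's Theme table.
; PaintValidate caps relative corner height; optional debug text shows grid index.
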(event `self.ReceiveBeginPlay`)

(event `self.ReceiveTick`
  (params (DeltaSeconds :type "Float (single-precision)")))

(fn `ChangeHightness`
  (params (Point :type "Actor Object Reference"))
  (bind _keys (`BlueprintMapLibrary.Map_Keys` (`self.Points`)))
  (for _array_element _keys
    (if (== (`BlueprintMapLibrary.Map_Find` (`self.Points`) _array_element) (`local.Point`))
      (`BlueprintMapLibrary.Map_Add` (`self.Hightness`) _array_element (+ (`BlueprintMapLibrary.Map_Find` (`self.Hightness`) _array_element) 1))))
  (`self.UpdateHightness` (`self.Hightness`))
  (`self.UpdateMesh`))

(fn `MakeCornerRowName`
  (params (Key0 :type "/Game/Blueprints/SceneBuild/EN_TileCorners Enum" :default "NewEnumerator0") (Key1 :type "/Game/Blueprints/SceneBuild/EN_TileCorners Enum" :default "NewEnumerator0") (Key2 :type "/Game/Blueprints/SceneBuild/EN_TileCorners Enum" :default "NewEnumerator0") (Key3 :type "/Game/Blueprints/SceneBuild/EN_TileCorners Enum" :default "NewEnumerator0") (TargetMap :type "Map of /Game/Blueprints/SceneBuild/EN_TileCorners Enum to Integer (by ref)"))
  (returns (ReturnValue :type Name))
  (return (`KismetStringLibrary.Conv_StringToName` (`KismetStringLibrary.Concat_StrStr` (`KismetStringLibrary.Conv_IntToString` (`BlueprintMapLibrary.Map_Find` TargetMap Key0)) (`KismetStringLibrary.Conv_IntToString` (`BlueprintMapLibrary.Map_Find` TargetMap Key1)) (`KismetStringLibrary.Conv_IntToString` (`BlueprintMapLibrary.Map_Find` TargetMap Key2)) (`KismetStringLibrary.Conv_IntToString` (`BlueprintMapLibrary.Map_Find` TargetMap Key3))))))

(fn `PaintValidate`
  (params (Point :type "Actor Object Reference"))
  (returns (CanPaintUp :type Boolean))
  (locals (TileCorner :type "/Game/Blueprints/SceneBuild/EN_TileCorners Enum"))
  (bind _keys (`BlueprintMapLibrary.Map_Keys` (`self.Points`)))
  (for _array_element _keys
    (if (== (`BlueprintMapLibrary.Map_Find` (`self.Points`) _array_element) (`local.Point`))
      (set `local.TileCorner` _array_element)))
  (if (< (`BlueprintMapLibrary.Map_Find` (`self.Hightness`) (`local.TileCorner`)) 3)
    (return true)
    (else
      (return false))))

(fn `Show Debug`
  (bind (_index_x _index_y) (break `IntPoint` (`self.Index`)))
  (if (`self.IsDebugging`)
    (`TextRenderComponent.K2_SetText` (`self.Text_ID`) (`|FormatText` "{X}/{Y}" _index_x _index_y))
    (bind _values (`BlueprintMapLibrary.Map_Values` (`self.Hightness`)))
    (`SceneComponent.K2_SetRelativeLocation` (`self.Text_ID`) (`KismetMathLibrary.MakeVector` 0.0 0.0 (`KismetMathLibrary.Conv_IntToDouble` (+ (* (+ (`.MaxValue` (`KismetMathLibrary.MaxOfIntArray` _values)) (`self.ActorHight`)) 50) 5))) false false)))

(fn `UpdateHightness`
  (params (TargetMap :type "Map of /Game/Blueprints/SceneBuild/EN_TileCorners Enum to Integer (by ref)"))
  (locals (Min :type Integer :default 999))
  (bind _targetmap (`local.TargetMap`))
  (bind _values (`BlueprintMapLibrary.Map_Values` TargetMap))
  (set `local.Min` (`.MinValue` (`KismetMathLibrary.MinOfIntArray` _values)))
  (if (!= (`local.Min`) 0)
    (bind _keys (`BlueprintMapLibrary.Map_Keys` (`local.TargetMap`)))
    (for _array_element _keys
      (`BlueprintMapLibrary.Map_Add` _targetmap _array_element (- (`BlueprintMapLibrary.Map_Find` _targetmap _array_element) (`local.Min`))))
    (`SceneComponent.K2_AddLocalOffset` (`self.Tile`) (`KismetMathLibrary.MakeVector` 0.0 0.0 (* (`local.Min`) 50.0)) false false)
    (set `self.ActorHight` (+ (`self.ActorHight`) (`local.Min`)))))

(fn `UpdateMesh`
  (returns (Success :type Boolean))
  (bind _returnvalue (`self.MakeCornerRowName` "NewEnumerator1" "NewEnumerator3" "NewEnumerator2" "NewEnumerator0" (`self.Hightness`)))
  (bind _returnvalue_2 (`|GetDataTableRow` (`self.ProxyMeshDT`) _returnvalue)
    (:`then`
      (bind (_proxymesh _rotation) (break `/Game/Blueprints/SceneBuild/Structures/ST_ProxyMappingMesh` _returnvalue_2))
      (bind _returnvalue_3 (`|GetDataTableRow` (`/Game/Blueprints/GameBlueprints/BP_CameraPawn.Theme` (cast `/Game/Blueprints/GameBlueprints/BP_CameraPawn` (`GameplayStatics.GetPlayerPawn` 0) :!pure true)) (`KismetStringLibrary.Conv_StringToName` _proxymesh))
        (:`then`
          (`StaticMeshComponent.SetStaticMesh` (`self.Tile`) (`.Mesh_2_E9CE701A4AB9148ADF33E0AF7F4D3A34` (break `/Game/Blueprints/SceneBuild/Structures/ST_Theme_SM` _returnvalue_3)))
          (`SceneComponent.K2_SetRelativeRotation` (`self.Tile`) (`KismetMathLibrary.MakeRotator` 0.0 0.0 (* -1 _rotation)) false false)
          (`self.Show Debug`)
          (return true))))
    (:`RowNotFound`
      (`KismetSystemLibrary.PrintString` (`KismetStringLibrary.Concat_StrStr` "//////////////////////" (`KismetStringLibrary.Conv_NameToString` _returnvalue) "//////////////////////"))
      (return false))))

(fn `UserConstructionScript`
  (`SceneComponent.SetVisibility` (`self.DebugActor`) (`self.IsDebugging`) true))