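; BP_SceneBuild_Main builds a grid map at BeginPlay from child actors for tiles, corner points and inner edges.
; Tiles and points are stored in index-keyed maps, then cross-linked so each tile knows its four corners and each point its neighbouring tiles.
; Edges sit between adjacent tiles, but both orientations share index keys in MapEdgesData, so later entries overwrite earlier ones.
; An unconnected node would run a Python map-export script.
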(event `self.ReceiveBeginPlay`
  (`self.BuildMap`))

(event `BuildMap`
  (`self.MakeMapTiles`)
  (`self.MakeMapPoints`)
  (`self.JoinPointsWithTiles`)
  (`self.MakeMapEdges_LeftRight`)
  (`self.MakeMapEdges_UpDown`))

(fn `FindPoint`
  (params (TargetMap :type "Map of IntPoint Structure to /Game/Blueprints/SceneBuild/BP_MapPoint Object Reference (by ref)") (IntPoint :type "IntPoint Structure (by ref)") (Offset :type "IntPoint Structure (by ref)"))
  (returns (Value :type "/Game/Blueprints/SceneBuild/BP_MapPoint Object Reference"))
  (bind (_x _y) (break `IntPoint` Offset))
  (bind (_x_2 _y_2) (break `IntPoint` IntPoint))
  (return (`BlueprintMapLibrary.Map_Find` TargetMap (make `IntPoint` (+ _x_2 _x) (+ _y_2 _y)))))

(fn `GetTileLocation`
  (params (X :type Integer) (Y :type Integer) (Destance :type "Float (double-precision)") (`Location Z` :type "Float (double-precision)"))
  (returns (Location :type "Vector Structure"))
  (bind _returnvalue (/ Destance 2.0))
  (return (`KismetMathLibrary.MakeVector` (+ (* X Destance) _returnvalue) (+ (* Y Destance) _returnvalue) `Location Z`)))

(fn `JoinPointsWithTiles`
  (bind _keys (`BlueprintMapLibrary.Map_Keys` (`self.MapTilesData`)))
  (for _array_element _keys
    (`|ExecutionSequence`
      (:`then_0`
        (bind _value (`BlueprintMapLibrary.Map_Find` (`self.MapTilesData`) _array_element))
        (bind _points (`/Game/Blueprints/SceneBuild/BP_MapTile.Points` _value))
        (bind _value_2 (`self.FindPoint` (`self.MapPointsData`) _array_element (make `IntPoint` 0)))
        (`BlueprintMapLibrary.Map_Add` _points "NewEnumerator0" _value_2)
        (`BlueprintMapLibrary.Map_Add` (`/Game/Blueprints/SceneBuild/BP_MapPoint.Tiles` _value_2) "NewEnumerator3" _value))
      (:`then_1`
        (bind _value_3 (`self.FindPoint` (`self.MapPointsData`) _array_element (make `IntPoint` 1)))
        (`BlueprintMapLibrary.Map_Add` _points "NewEnumerator1" _value_3)
        (`BlueprintMapLibrary.Map_Add` (`/Game/Blueprints/SceneBuild/BP_MapPoint.Tiles` _value_3) "NewEnumerator2" _value))
      (:`then_2`
        (bind _value_4 (`self.FindPoint` (`self.MapPointsData`) _array_element (make `IntPoint` 0 1)))
        (`BlueprintMapLibrary.Map_Add` _points "NewEnumerator2" _value_4)
        (`BlueprintMapLibrary.Map_Add` (`/Game/Blueprints/SceneBuild/BP_MapPoint.Tiles` _value_4) "NewEnumerator1" _value))
      (:`then_3`
        (bind _value_5 (`self.FindPoint` (`self.MapPointsData`) _array_element (make `IntPoint` 1 1)))
        (`BlueprintMapLibrary.Map_Add` _points "NewEnumerator3" _value_5)
        (`BlueprintMapLibrary.Map_Add` (`/Game/Blueprints/SceneBuild/BP_MapPoint.Tiles` _value_5) "NewEnumerator0" _value)))))

(fn `MakeMapEdges_LeftRight`
  (locals (Index_X :type Integer) (Index_Y :type Integer))
  (bind (_size_x _size_y) (break `IntPoint` (`self.Size`)))
  (bind _celldestance (`self.CellDestance`))
  (bind _size_x_2 (break `IntPoint` (`self.Size`)))
  (bind (_location_x _location_y _location_z) (`KismetMathLibrary.BreakVector` (`self.GetTileLocation` (`local.Index_X`) (`local.Index_Y`) _celldestance)))
  (bind _intpoint (make `IntPoint` (`local.Index_X`) (`local.Index_Y`)))
  (for _index (range (+ (- _size_x_2 2) 1))
    (set `local.Index_X` _index)
    (for _index_2 (range _size_y)
      (set `local.Index_Y` _index_2)
      (bind _returnvalue (`AddComponent|NODE_AddChildActorComponent-2` :`RelativeTransform` (`KismetMathLibrary.MakeTransform` (`KismetMathLibrary.MakeVector` (+ _location_x (/ _celldestance 2.0)) _location_y _location_z) (struct :`Pitch` 90.0))))
      (bind _asbp_map_edge (cast `/Game/Blueprints/SceneBuild/BP_MapEdge` (`ChildActorComponent.ChildActor` _returnvalue) :!pure true))
      (set `/Game/Blueprints/SceneBuild/BP_MapEdge.Index` _intpoint _asbp_map_edge)
      (`BlueprintMapLibrary.Map_Add` (`self.MapEdgesData`) _intpoint _asbp_map_edge))))

(fn `MakeMapEdges_UpDown`
  (locals (Index_X :type Integer) (Index_Y :type Integer))
  (bind (_size_x _size_y) (break `IntPoint` (`self.Size`)))
  (bind _celldestance (`self.CellDestance`))
  (bind _size_x_2 (break `IntPoint` (`self.Size`)))
  (bind (_location_x _location_y _location_z) (`KismetMathLibrary.BreakVector` (`self.GetTileLocation` (`local.Index_X`) (`local.Index_Y`) _celldestance)))
  (bind _intpoint (make `IntPoint` (`local.Index_X`) (`local.Index_Y`)))
  (for _index (range _size_x_2)
    (set `local.Index_X` _index)
    (for _index_2 (range (+ (- _size_y 2) 1))
      (set `local.Index_Y` _index_2)
      (bind _returnvalue (`AddComponent|NODE_AddChildActorComponent-3` :`RelativeTransform` (`KismetMathLibrary.MakeTransform` (`KismetMathLibrary.MakeVector` _location_x (+ _location_y (/ _celldestance 2.0)) _location_z) (struct :`Roll` -90.0))))
      (bind _asbp_map_edge (cast `/Game/Blueprints/SceneBuild/BP_MapEdge` (`ChildActorComponent.ChildActor` _returnvalue) :!pure true))
      (set `/Game/Blueprints/SceneBuild/BP_MapEdge.Index` _intpoint _asbp_map_edge)
      (`BlueprintMapLibrary.Map_Add` (`self.MapEdgesData`) _intpoint _asbp_map_edge))))

(fn `MakeMapPoints`
  (locals (Map_Data :type String))
  (bind (_size_x _size_y) (break `IntPoint` (`self.Size`)))
  (bind _celldestance (`self.CellDestance`))
  (bind _size_x_2 (break `IntPoint` (`self.Size`)))
  (for _index (range (+ _size_x_2 1))
    (for _index_2 (range (+ _size_y 1))
      (bind _returnvalue (`AddComponent|NODE_AddChildActorComponent-0` :`RelativeTransform` (`KismetMathLibrary.MakeTransform` (`KismetMathLibrary.MakeVector` (* _index _celldestance) (* _index_2 _celldestance)))))
      (bind _asbp_map_point (cast `/Game/Blueprints/SceneBuild/BP_MapPoint` (`ChildActorComponent.ChildActor` _returnvalue) :!pure true))
      (bind _output_get (set `/Game/Blueprints/SceneBuild/BP_MapPoint.Index` (make `IntPoint` _index _index_2) _asbp_map_point))
      (`BlueprintMapLibrary.Map_Add` (`self.MapPointsData`) _output_get _asbp_map_point))))

(fn `MakeMapTiles`
  (locals (Index_X :type Integer) (Index_Y :type Integer))
  (bind (_size_x _size_y) (break `IntPoint` (`self.Size`)))
  (bind _size_x_2 (break `IntPoint` (`self.Size`)))
  (bind _intpoint (make `IntPoint` (`local.Index_X`) (`local.Index_Y`)))
  (for _index (range _size_x_2)
    (set `local.Index_X` _index)
    (for _index_2 (range _size_y)
      (set `local.Index_Y` _index_2)
      (bind _returnvalue (`AddComponent|NODE_AddChildActorComponent-1` :`RelativeTransform` (`KismetMathLibrary.MakeTransform` (`self.GetTileLocation` (`local.Index_X`) (`local.Index_Y`) (`self.CellDestance`)))))
      (bind _asbp_map_tile (cast `/Game/Blueprints/SceneBuild/BP_MapTile` (`ChildActorComponent.ChildActor` _returnvalue) :!pure true))
      (set `/Game/Blueprints/SceneBuild/BP_MapTile.Index` _intpoint _asbp_map_tile)
      (`BlueprintMapLibrary.Map_Add` (`self.MapTilesData`) _intpoint _asbp_map_tile)
      (`/Game/Blueprints/SceneBuild/BP_MapTile.Show Debug` _asbp_map_tile))))

(fn `UserConstructionScript`)